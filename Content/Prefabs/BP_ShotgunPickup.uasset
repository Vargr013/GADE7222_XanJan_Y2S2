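; Shotgun pickup that bobs on a sine wave around its starting height until flagged as picked up.
; OnPickedUp queries the collector through BPI_Inventory, setting ammo if the current weapon matches ShotgunClass, otherwise only flagging the pickup as collected.
; GetPickupType reports its weapon type.
; The overlap event is empty, and older BP_MainCharacter logic for spawning the shotgun, refilling and destroying the pickup is disconnected.
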(event `self.ReceiveBeginPlay`
  (bind (_returnvalue_x _returnvalue_y _returnvalue_z) (`KismetMathLibrary.BreakVector` (`SceneComponent.K2_GetComponentLocation` (`self.ShotgunMesh`))))
  ; Initalise
  (set `self.InitialZ` _returnvalue_z))

(event `self.ReceiveTick`
  (params (DeltaSeconds :type "Float (single-precision)"))
  (bind (_returnvalue_x _returnvalue_y) (`KismetMathLibrary.BreakVector` (`SceneComponent.K2_GetComponentLocation` (`self.ShotgunMesh`))))
  ; Pickup Bouncing Logic
  (if (not (`self.HasBeenPickedUp`))
    (`SceneComponent.K2_SetWorldLocation` (`self.ShotgunMesh`) (`KismetMathLibrary.MakeVector` _returnvalue_x _returnvalue_y (+ (* (`KismetMathLibrary.Sin` (* (`KismetSystemLibrary.GetGameTimeInSeconds`) (`self.BounceSpeed`))) (`self.BounceHeight`)) (`self.InitialZ`))) false false)))

(event `self.PickupCollison.OnComponentBeginOverlap`
  (params (OverlappedComponent :type "PrimitiveComponent Object Reference") (OtherActor :type "Actor Object Reference") (OtherComp :type "PrimitiveComponent Object Reference") (OtherBodyIndex :type Integer) (bFromSweep :type Boolean) (SweepResult :type "HitResult Structure (by ref)"))
  ; Pickup Shotgun Logic
)

(event `/Game/Blueprints/Interfaces/BPI_Pickupable.OnPickedUp`
  (params (Collector :type "Actor Object Reference"))
  (if (`KismetSystemLibrary.DoesImplementInterface` Collector "/Game/Blueprints/Interfaces/BPI_Inventory.BPI_Inventory_C")
    (bind _equipedweapon (message `/Game/Blueprints/Interfaces/BPI_Inventory.GetCurrentWeapon` Collector))
    (if (== _equipedweapon (`self.ShotgunClass`))
      (bind _asbp_shotgun (cast `/Game/Blueprints/Weapons/BP_Shotgun` _equipedweapon))
      (set `/Game/Blueprints/Weapons/BP_WeaponBase.Ammo` 2 _asbp_shotgun)
      (else
        (set `self.HasBeenPickedUp` true)))))

(fn `GetPickupType`
  (returns (PickupType :type String))
  (return (`self.WeaponType`)))

(fn `UserConstructionScript`)