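; BP_GameMode is the game mode that runs a five-minute match countdown and ends the game when time runs out.
; BeginPlay sets the remaining time and starts a looping one-second timer event that decrements it.
; At zero, OnMatchEnd pauses the game and prints a debug string, then the timer is cleared and BP_MainCharacter on player 0 shows the game-over screen.
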(event `self.ReceiveBeginPlay`
  ; Timer Logic
  (set `self.MatchTimeRemaining` 300.0)
  (bind _returnvalue (`KismetSystemLibrary.K2_SetTimerDelegate` (delegate `TickMatchTimer`) 1.0 true)))

(event `TickMatchTimer`
  ; Timer Logic
  (set `self.MatchTimeRemaining` (- (`self.MatchTimeRemaining`) 1.0))
  (if (<= (`self.MatchTimeRemaining`) 0.0)
    (`self.OnMatchEnd`)
    (`KismetSystemLibrary.K2_ClearAndInvalidateTimerHandle` (stale `self.ReceiveBeginPlay` _returnvalue))
    (bind _asbp_main_character (cast `/Game/Blueprints/Character/BP_MainCharacter` (`GameplayStatics.GetPlayerCharacter` 0)))
    (`/Game/Blueprints/Character/BP_MainCharacter.Show Game Over Screen` _asbp_main_character)))

(fn `OnMatchEnd`
  (`GameplayStatics.SetGamePaused` true)
  (`KismetSystemLibrary.PrintString` "Klaar"))

(fn `UserConstructionScript`)