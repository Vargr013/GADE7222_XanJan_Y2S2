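; Player character Blueprint that handles Enhanced Input movement, camera look, jumping, sprinting and weapon use.
; On BeginPlay it adds the IMC_Player mapping context, initialises speed and health, then spawns a shovel at the camera's transform as the current weapon.
; Sprint raises walk speed and a forward/back input multiplier until released.
; Fire calls FireWeapon on the current weapon and prints debug text.
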(event `self.ReceiveBeginPlay`
  ; Allow Player Movement
  (bind _asplayer_controller (cast `PlayerController` (`self.GetController`)))
  (bind _returnvalue (pcsubsystem `EnhancedInputLocalPlayerSubsystem` _asplayer_controller))
  (`/Engine/EditorBlueprintResources/StandardMacros.IsValid` _returnvalue
    (:`Is Valid`
      (`EnhancedInputSubsystemInterface.AddMappingContext` _returnvalue "/Game/Input/IMC_Player.IMC_Player" 0 (struct))
      (`self.Initialise`)
      (`self.SpawnShovel`))))

(event `EnhancedInput|/Game/Input/Actions/IA_Look`
  (params (ActionValue :type "Vector2D Structure") (ElapsedSeconds :type "Float (double-precision)") (TriggeredSeconds :type "Float (double-precision)") (InputAction :type "InputAction Object Reference" :default "/Game/Input/Actions/IA_Look.IA_Look"))
  ; Camera Input Logic
  (:`Triggered`
    (`self.AddControllerYawInput` ActionValue_X)
    (`self.AddControllerPitchInput` (* ActionValue_Y -1.0))))

(event `EnhancedInput|/Game/Input/Actions/IA_Jump`
  (params (ActionValue :type Boolean) (ElapsedSeconds :type "Float (double-precision)") (TriggeredSeconds :type "Float (double-precision)") (InputAction :type "InputAction Object Reference" :default "/Game/Input/Actions/IA_Jump.IA_Jump"))
  ; Jump Logic
  (:`Triggered`
    (`self.Jump`))
  (:`Completed`
    (`self.StopJumping`)))

(event `EnhancedInput|/Game/Input/Actions/IA_Move`
  (params (ActionValue :type "Vector2D Structure") (ElapsedSeconds :type "Float (double-precision)") (TriggeredSeconds :type "Float (double-precision)") (InputAction :type "InputAction Object Reference" :default "/Game/Input/Actions/IA_Move.IA_Move"))
  (bind (_returnvalue_roll _returnvalue_pitch _returnvalue_yaw) (`KismetMathLibrary.BreakRotator` (`self.GetControlRotation`)))
  (bind (_returnvalue_roll_2 _returnvalue_pitch_2 _returnvalue_yaw_2) (`KismetMathLibrary.BreakRotator` (`self.GetControlRotation`)))
  ; Movement Logic
  (:`Triggered`
    (`self.AddMovementInput` (`KismetMathLibrary.GetRightVector` (`KismetMathLibrary.MakeRotator` _returnvalue_roll 0.0 _returnvalue_yaw)) ActionValue_X)
    (`self.AddMovementInput` (`KismetMathLibrary.GetForwardVector` (`KismetMathLibrary.MakeRotator` 0.0 0.0 _returnvalue_yaw_2)) (* ActionValue_Y (`self.Movement  Mult`)))))

(event `EnhancedInput|/Game/Input/Actions/IA_Sprint`
  (params (ActionValue :type Boolean) (ElapsedSeconds :type "Float (double-precision)") (TriggeredSeconds :type "Float (double-precision)") (InputAction :type "InputAction Object Reference" :default "/Game/Input/Actions/IA_Sprint.IA_Sprint"))
  ; Sprint logic
  (:`Triggered`
    (set `CharacterMovementComponent.MaxWalkSpeed` 950.0 (`self.CharacterMovement`))
    (set `self.Movement  Mult` 3))
  (:`Completed`
    (set `CharacterMovementComponent.MaxWalkSpeed` 500.0 (`self.CharacterMovement`))
    (set `self.Movement  Mult` 1)))

(event `EnhancedInput|/Game/Input/Actions/IA_Fire`
  (params (ActionValue :type Boolean) (ElapsedSeconds :type "Float (double-precision)") (TriggeredSeconds :type "Float (double-precision)") (InputAction :type "InputAction Object Reference" :default "/Game/Input/Actions/IA_Fire.IA_Fire"))
  (bind _current_weapon (`self.Current Weapon`))
  ; Fire Weapon Logic
  (:`Triggered`
    (`/Engine/EditorBlueprintResources/StandardMacros.IsValid` _current_weapon
      (:`Is Valid`
        (`/Game/Blueprints/Weapons/BP_WeaponBase.FireWeapon` _current_weapon)
        (`KismetSystemLibrary.PrintText` "Boom!")))))

(fn `Initialise`
  ; Movement
  (set `self.Movement  Mult` 1)
  (set `CharacterMovementComponent.MaxWalkSpeed` 500.0 (`self.CharacterMovement`))
  ; Health
  (set `self.Health` 100))

(fn `SpawnShovel`
  (bind _returnvalue (`|SpawnActorFromClass` "/Game/Blueprints/Weapons/BP_Shovel.BP_Shovel_C" (`SceneComponent.GetSocketTransform` (`self.Camera`) "None" "RTS_World") "Undefined" "MultiplyWithRoot" null null))
  (bind _output_get (set `self.ShovelRef` _returnvalue))
  (set `self.Current Weapon` _output_get))

(fn `UserConstructionScript`)