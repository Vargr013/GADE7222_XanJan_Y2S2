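; Player character with Enhanced Input movement, sprint, pause menu and health, using a shovel and a pickup-unlocked shotgun.
; Weapon swaps spawn fresh actors on mesh sockets; firing traces from the camera via interface messages, with an empty weapon reverting to the shovel.
; Pickups arrive through capsule overlap.
; Death credits the killer on the GameMode leaderboard, removes the HUD, messages spawners to respawn and shows a pausing game-over screen.
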(event `Key|H`
  (params (Key :type "Key Structure"))
  ; Test Health Bar
  (:`Pressed`
    (`/Game/Blueprints/Interfaces/BPI_Damageable.TakeDamage` 25.0)))

(event `self.ReceiveBeginPlay`
  ; Allow Player Movement
  (`|ExecutionSequence`
    (:`then_0`
      (bind _asplayer_controller (cast `PlayerController` (`self.GetController`)))
      (bind _returnvalue (pcsubsystem `EnhancedInputLocalPlayerSubsystem` _asplayer_controller))
      (`/Engine/EditorBlueprintResources/StandardMacros.IsValid` _returnvalue
        (:`Is Valid`
          (`EnhancedInputSubsystemInterface.AddMappingContext` _returnvalue "/Game/Input/IMC_Player.IMC_Player" 0 (struct))
          (`self.Initialise`))))))

(event `EnhancedInput|/Game/Input/Actions/IA_Look`
  (params (ActionValue :type "Vector2D Structure") (ElapsedSeconds :type "Float (double-precision)") (TriggeredSeconds :type "Float (double-precision)") (InputAction :type "InputAction Object Reference" :default "/Game/Input/Actions/IA_Look.IA_Look"))
  ; Camera Input Logic
  (:`Triggered`
    (`self.AddControllerYawInput` ActionValue_X)
    (`self.AddControllerPitchInput` (* ActionValue_Y -1.0))))

(event `EnhancedInput|/Game/Input/Actions/IA_Jump`
  (params (ActionValue :type Boolean) (ElapsedSeconds :type "Float (double-precision)") (TriggeredSeconds :type "Float (double-precision)") (InputAction :type "InputAction Object Reference" :default "/Game/Input/Actions/IA_Jump.IA_Jump"))
  ; Jump Logic
  (:`Triggered`
    (`self.Jump`))
  (:`Completed`
    (`self.StopJumping`)))

(event `EnhancedInput|/Game/Input/Actions/IA_Move`
  (params (ActionValue :type "Vector2D Structure") (ElapsedSeconds :type "Float (double-precision)") (TriggeredSeconds :type "Float (double-precision)") (InputAction :type "InputAction Object Reference" :default "/Game/Input/Actions/IA_Move.IA_Move"))
  (bind (_returnvalue_roll _returnvalue_pitch _returnvalue_yaw) (`KismetMathLibrary.BreakRotator` (`self.GetControlRotation`)))
  (bind (_returnvalue_roll_2 _returnvalue_pitch_2 _returnvalue_yaw_2) (`KismetMathLibrary.BreakRotator` (`self.GetControlRotation`)))
  ; Movement Logic
  (:`Triggered`
    (`self.AddMovementInput` (`KismetMathLibrary.GetRightVector` (`KismetMathLibrary.MakeRotator` _returnvalue_roll 0.0 _returnvalue_yaw)) ActionValue_X)
    (`self.AddMovementInput` (`KismetMathLibrary.GetForwardVector` (`KismetMathLibrary.MakeRotator` 0.0 0.0 _returnvalue_yaw_2)) (* ActionValue_Y (`self.Movement  Mult`)))))

(event `EnhancedInput|/Game/Input/Actions/IA_Sprint`
  (params (ActionValue :type Boolean) (ElapsedSeconds :type "Float (double-precision)") (TriggeredSeconds :type "Float (double-precision)") (InputAction :type "InputAction Object Reference" :default "/Game/Input/Actions/IA_Sprint.IA_Sprint"))
  ; Sprint logic
  (:`Triggered`
    (set `CharacterMovementComponent.MaxWalkSpeed` 950.0 (`self.CharacterMovement`))
    (set `self.Movement  Mult` 3))
  (:`Completed`
    (set `CharacterMovementComponent.MaxWalkSpeed` 500.0 (`self.CharacterMovement`))
    (set `self.Movement  Mult` 1)))

(event `EnhancedInput|/Game/Input/Actions/IA_Fire`
  (params (ActionValue :type Boolean) (ElapsedSeconds :type "Float (double-precision)") (TriggeredSeconds :type "Float (double-precision)") (InputAction :type "InputAction Object Reference" :default "/Game/Input/Actions/IA_Fire.IA_Fire"))
  (bind _current_weapon (`self.Current Weapon`))
  (bind _current_weapon_2 (`self.Current Weapon`))
  (bind _playercameramanager (`PlayerController.PlayerCameraManager` (`self.Player Ref`)))
  (bind _returnvalue (`PlayerCameraManager.GetCameraLocation` _playercameramanager))
  ; Fire Weapon Logic
  (:`Triggered`
    (if (== _current_weapon (`self.ShovelRef`))
      (set `self.Weapon1Fired` true)
      (`KismetSystemLibrary.Delay` 1.0)
      (set `self.Player Ref` (`GameplayStatics.GetPlayerController` 0) :!label _label)
      (bind _range (message `/Game/Blueprints/Interfaces/BPI_Shootable.GetRange` (`self.Current Weapon`)))
      (message `/Game/Blueprints/Interfaces/BPI_Shootable.Fire` (`self.Current Weapon`) _returnvalue (+ _returnvalue (* (`SceneComponent.GetForwardVector` (`PlayerCameraManager.TransformComponent` _playercameramanager)) _range)) (`self.Player Ref`))
      (set `self.Weapon1Fired` false)
      (set `self.Weapon2Fired` false)
      (bind _currentammo (message `/Game/Blueprints/Interfaces/BPI_Shootable.GetCurrentAmmo` _current_weapon_2))
      (bind _result (`/Engine/EditorBlueprintResources/StandardMacros.DecrementInt` _currentammo)
        (:`  `
          (message `/Game/Blueprints/Interfaces/BPI_Shootable.SetAmmo` _current_weapon_2 _result)))
      (else
        (bind _currentammo_2 (message `/Game/Blueprints/Interfaces/BPI_Shootable.GetCurrentAmmo` _current_weapon))
        (if (> _currentammo_2 0)
          (set `self.Weapon2Fired` true)
          (`KismetSystemLibrary.Delay` 0.2)
          (goto _label)
          (else
            (`self.SpawnShovel`)))))))

(event `EnhancedInput|/Game/Input/Actions/IA_Shovel`
  (params (ActionValue :type Boolean) (ElapsedSeconds :type "Float (double-precision)") (TriggeredSeconds :type "Float (double-precision)") (InputAction :type "InputAction Object Reference" :default "/Game/Input/Actions/IA_Shovel.IA_Shovel"))
  ; Swap To Shovel
  (:`Triggered`
    (`self.SpawnShovel`)))

(event `/Game/Blueprints/Interfaces/BPI_Damageable.TakeDamage`
  (params (DamageAmount :type "Float (double-precision)") (DamageCauser :type "Actor Object Reference"))
  ; TakeDamage
  (bind _output_get (set `self.Health` (- (`self.Health`) DamageAmount)))
  (if (<= (`KismetMathLibrary.Clamp` (`KismetMathLibrary.FTrunc` _output_get) 0 100) 0)
    (set `self.Dead` true)
    (`self.UpdateLeaderboard` self DamageCauser)
    (`/Engine/EditorBlueprintResources/StandardMacros.IsValid` (`Controller.K2_GetPawn` (`GameplayStatics.GetPlayerController` 0))
      (:`Is Valid`
        (`self.OnDeath`)
        (bind _outactors (`GameplayStatics.GetAllActorsWithInterface` "/Game/Blueprints/Interfaces/BPI_Spawner.BPI_Spawner_C"))
        (message `/Game/Blueprints/Interfaces/BPI_Spawner.RespawnInitiate` _outactors self)
        (`self.Show Game Over Screen`)))))

(event `EnhancedInput|/Game/Input/Actions/IA_Shotgun`
  (params (ActionValue :type Boolean) (ElapsedSeconds :type "Float (double-precision)") (TriggeredSeconds :type "Float (double-precision)") (InputAction :type "InputAction Object Reference" :default "/Game/Input/Actions/IA_Shotgun.IA_Shotgun"))
  ; Swap To Shotgun
  (:`Triggered`
    (if (`self.UnlockedShotgun`)
      (`self.SpawnDBShotgun`))))

(event `self.CapsuleComponent.OnComponentBeginOverlap`
  (params (OverlappedComponent :type "PrimitiveComponent Object Reference") (OtherActor :type "Actor Object Reference") (OtherComp :type "PrimitiveComponent Object Reference") (OtherBodyIndex :type Integer) (bFromSweep :type Boolean) (SweepResult :type "HitResult Structure (by ref)"))
  (if (`KismetSystemLibrary.DoesImplementInterface` OtherActor "/Game/Blueprints/Interfaces/BPI_Pickupable.BPI_Pickupable_C")
    (bind _pickuptype (message `/Game/Blueprints/Interfaces/BPI_Pickupable.GetPickupType` OtherActor))
    (if (`KismetStringLibrary.EqualEqual_StrStr` _pickuptype (`self.ShotGunPickupName`))
      (message `/Game/Blueprints/Interfaces/BPI_Pickupable.OnPickedUp` (`self.Player Ref`) self)
      (`self.SpawnDBShotgun`)
      (`KismetSystemLibrary.Delay` 0.5)
      (`self.K2_DestroyActor` OtherActor)
      (else
        (message `/Game/Blueprints/Interfaces/BPI_Pickupable.OnPickedUp` OtherActor self)))))

(event `/Game/Blueprints/Interfaces/BPI_Damageable.AddHealth`
  (params (HealingAmount :type "Float (double-precision)"))
  (set `self.Health` (`KismetMathLibrary.FClamp` (+ (`self.Health`) HealingAmount) 0.0 100.0)))

(event `EnhancedInput|/Game/Input/Actions/IA_PauseGame`
  (params (ActionValue :type Boolean) (ElapsedSeconds :type "Float (double-precision)") (TriggeredSeconds :type "Float (double-precision)") (InputAction :type "InputAction Object Reference" :default "/Game/Input/Actions/IA_PauseGame.IA_PauseGame"))
  (bind _returnvalue (`GameplayStatics.GetPlayerController` 0))
  ; Pause Game
  (:`Started`
    (if (not (`self.IsPauseMenuOpen`))
      (set `self.IsPauseMenuOpen` true)
      (bind _returnvalue_2 (`|CreateWidget` "/Game/UI/WBP_MenuPause.WBP_MenuPause_C" _returnvalue))
      (bind _output_get (set `self.PauseMenuWidget` _returnvalue_2))
      (`UserWidget.AddToViewport` _output_get 0)
      (`WidgetBlueprintLibrary.SetInputMode_GameAndUIEx` _returnvalue (`self.PauseMenuWidget`))
      (set `PlayerController.bShowMouseCursor` true (`GameplayStatics.GetPlayerController` 0))
      (`GameplayStatics.SetGamePaused` true)
      (else
        (set `self.IsPauseMenuOpen` false)
        (`Widget.RemoveFromParent` (`self.PauseMenuWidget`))
        (`GameplayStatics.SetGamePaused` false)
        (`WidgetBlueprintLibrary.SetInputMode_GameOnly` (`GameplayStatics.GetPlayerController` 0))
        (set `PlayerController.bShowMouseCursor` false (`GameplayStatics.GetPlayerController` 0))))))

(event `Show Game Over Screen`
  (bind _returnvalue (`GameplayStatics.GetPlayerController` 0))
  ; Game Over
  (if (not (`self.IsGameOverOpen`))
    (set `self.IsGameOverOpen` true)
    (bind _returnvalue_2 (`|CreateWidget` "/Game/UI/WBP_MatchOver.WBP_MatchOver_C" _returnvalue))
    (bind _output_get (set `self.GameOverWidget` _returnvalue_2))
    (`UserWidget.AddToViewport` _output_get 0)
    (`WidgetBlueprintLibrary.SetInputMode_GameAndUIEx` _returnvalue (`self.GameOverWidget`))
    (set `PlayerController.bShowMouseCursor` true (`GameplayStatics.GetPlayerController` 0))
    (`GameplayStatics.SetGamePaused` true)
    (else
      (set `self.IsGameOverOpen` false)
      (`Widget.RemoveFromParent` (`self.GameOverWidget`))
      (`GameplayStatics.SetGamePaused` false)
      (`WidgetBlueprintLibrary.SetInputMode_GameOnly` (`GameplayStatics.GetPlayerController` 0))
      (set `PlayerController.bShowMouseCursor` false (`GameplayStatics.GetPlayerController` 0)))))

(fn `AddToLeaderboard`
  (params (CharacterToAdd :type "Actor Object Reference"))
  (if (`KismetSystemLibrary.DoesImplementInterface` CharacterToAdd "/Game/Blueprints/Interfaces/BPI_Damageable.BPI_Damageable_C")
    (bind _asbp_game_mode (cast `/Game/Levels/BP_GameMode` (`GameplayStatics.GetGameMode`)))
    (if (> (`/Game/Levels/BP_GameMode.MatchTimeRemaining` _asbp_game_mode) 290.0)
      (`KismetArrayLibrary.Array_Add` (`/Game/Levels/BP_GameMode.LeaderboardData` _asbp_game_mode) (make `/Game/Blueprints/Leaderboard/S_LeadboardEntry` (`self.PlayerName`))))))

(fn `CurrentHealth`
  (returns (Float :type "Float (double-precision)"))
  (return (`self.Health`)))

(fn `GetCharacterName`
  (returns (ReturnName :type String))
  (return (`self.PlayerName`)))

(fn `GetCurrentWeapon`
  (returns (EquipedWeapon :type "/Game/Blueprints/Weapons/BP_WeaponBase Object Reference"))
  (return null))

(fn `GetWeaponSocket`
  (returns (NewParam :type "Vector Structure"))
  (return (0.0 0.0 0.0)))

(fn `Initialise`
  ; Movement
  (set `self.Movement  Mult` 1)
  (set `CharacterMovementComponent.MaxWalkSpeed` 500.0 (`self.CharacterMovement`))
  ; Health
  (set `self.Health` 100.0)
  ; Display GUI to player
  (bind _returnvalue (`|CreateWidget` "/Game/UI/Widgets/W_HUD.W_HUD_C"))
  (bind _output_get (set `self.HudRef` _returnvalue))
  (`UserWidget.AddToViewport` _output_get 0)
  (`self.SpawnShovel`)
  (set `self.PlayerName` "Player")
  (`self.AddToLeaderboard` self))

(fn `isDead`
  (returns (bDead :type Boolean))
  (return (<= (`self.Health`) 0.0)))

(fn `OnDeath`
  (`Widget.RemoveFromParent` (`self.HudRef`))
  (`self.DisableInput` null))

(fn `Respawn`)

(fn `SpawnDBShotgun`
  (`self.K2_DestroyActor` (`self.Current Weapon`))
  (bind _returnvalue (`|SpawnActorFromClass` "/Game/Blueprints/Weapons/BP_Shotgun.BP_Shotgun_C" (`SceneComponent.GetSocketTransform` (`self.Mesh`) "DBSocket" "RTS_World") "Undefined" "MultiplyWithRoot" null null))
  (bind _output_get (set `self.ShotgunRef` _returnvalue))
  (`self.K2_AttachToComponent` _output_get (`self.Mesh`) "WeaponSocket" "SnapToTarget" "SnapToTarget" "SnapToTarget" true)
  (set `self.Current Weapon` (`self.ShotgunRef`))
  (set `self.UnlockedShotgun` true)
  (`SceneComponent.SetVisibility` (`Actor.RootComponent` (`self.Current Weapon`)) true true))

(fn `SpawnShovel`
  (if (`self.UnlockedShotgun`)
    (`self.K2_DestroyActor` (`self.Current Weapon`)))
  (bind _returnvalue (`|SpawnActorFromClass` "/Game/Blueprints/Weapons/BP_Shovel.BP_Shovel_C" (`SceneComponent.GetSocketTransform` (`self.Mesh`) "WeaponSocket" "RTS_World") "Undefined" "MultiplyWithRoot" null null))
  (`self.K2_AttachToComponent` _returnvalue (`self.Mesh`) "WeaponSocket" "SnapToTarget" "SnapToTarget" "SnapToTarget" true)
  (bind _output_get (set `self.ShovelRef` _returnvalue))
  (set `self.Current Weapon` _output_get)
  (`SceneComponent.SetVisibility` (`Actor.RootComponent` (`self.Current Weapon`)) true true))

(fn `UpdateLeaderboard`
  (params (KilledCharacter :type "Actor Object Reference") (KillerCharacter :type "Actor Object Reference"))
  (locals (`Killer Name` :type String))
  (bind _returnvalue (`GameplayStatics.GetGameMode`))
  (`/Engine/EditorBlueprintResources/StandardMacros.IsValid` _returnvalue
    (:`Is Valid`
      (bind _asbp_game_mode (cast `/Game/Levels/BP_GameMode` _returnvalue))
      (set `local.Killer Name` (`KismetSystemLibrary.GetObjectName` KillerCharacter))
      (bind _leaderboarddata (`/Game/Levels/BP_GameMode.LeaderboardData` _asbp_game_mode))
      (for (_array_element _array_index) _leaderboarddata
        (bind (_playername _kills) (break `/Game/Blueprints/Leaderboard/S_LeadboardEntry` _array_element))
        (if (`KismetStringLibrary.EqualEqual_StrStr` _playername (`local.Killer Name`))
          (bind _result (`/Engine/EditorBlueprintResources/StandardMacros.IncrementInt` _kills)
            (:`  `
              (`KismetArrayLibrary.Array_Set` _leaderboarddata _array_index (make `/Game/Blueprints/Leaderboard/S_LeadboardEntry` _playername _result))
              (break))))))))

(fn `UserConstructionScript`)