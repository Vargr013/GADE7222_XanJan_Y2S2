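; Base AI combat character that starts with a shovel, registers on the game mode's leaderboard and handles health, weapons and death.
; AI perception writes damageable actors to the blackboard's TargetActor key.
; Capsule overlaps collect interface-based pickups, with shotgun pickups replacing the held weapon, while firing sets timed per-weapon flags.
; Lethal damage credits the killer by object name, ragdolls the mesh, then messages BPI_Spawner actors to respawn it after a delay.
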(event `self.ReceiveBeginPlay`
  (`self.Initialise`))

(event `self.TakeDamage`
  (params (DamageAmount :type "Float (double-precision)") (DamageCauser :type "Actor Object Reference"))
  ; TakeDamage
  (bind _output_get (set `self.Health` (- (`self.Health`) DamageAmount)))
  (if (<= _output_get 0.0)
    (set `self.Dead` true)
    (`self.LeaderBoardUpdate` self DamageCauser)
    (`MovementComponent.StopMovementImmediately` (`self.CharacterMovement`))
    (`PrimitiveComponent.SetSimulatePhysics` (`self.Mesh`) true)
    (`KismetSystemLibrary.Delay` 1.0)
    (bind _outactors (`GameplayStatics.GetAllActorsWithInterface` "/Game/Blueprints/Interfaces/BPI_Spawner.BPI_Spawner_C"))
    (message `/Game/Blueprints/Interfaces/BPI_Spawner.RespawnInitiate` _outactors self)))

(event `self.AIPerception.OnTargetPerceptionUpdated`
  (params (Actor :type "Actor Object Reference") (Stimulus :type "AIStimulus Structure"))
  ; AI View
  (if (`KismetSystemLibrary.DoesImplementInterface` Actor "/Game/Blueprints/Interfaces/BPI_Damageable.BPI_Damageable_C")
    (`BlackboardComponent.SetValueAsObject` (`AIBlueprintHelperLibrary.GetBlackboard` null) "TargetActor" Actor)))

(event `self.CapsuleComponent.OnComponentBeginOverlap`
  (params (OverlappedComponent :type "PrimitiveComponent Object Reference") (OtherActor :type "Actor Object Reference") (OtherComp :type "PrimitiveComponent Object Reference") (OtherBodyIndex :type Integer) (bFromSweep :type Boolean) (SweepResult :type "HitResult Structure (by ref)"))
  ; Pickup Implementation
  (if (`KismetSystemLibrary.DoesImplementInterface` OtherActor "/Game/Blueprints/Interfaces/BPI_Pickupable.BPI_Pickupable_C")
    (bind _pickuptype (message `/Game/Blueprints/Interfaces/BPI_Pickupable.GetPickupType` OtherActor))
    (if (`KismetStringLibrary.EqualEqual_StrStr` _pickuptype (`self.Shot Gun Pickup name`))
      (message `/Game/Blueprints/Interfaces/BPI_Pickupable.OnPickedUp` OtherActor self)
      (`self.SpawnDBShotgun`)
      (else
        (message `/Game/Blueprints/Interfaces/BPI_Pickupable.OnPickedUp` OtherActor self)))
    (`KismetSystemLibrary.Delay` 0.5)
    (`self.K2_DestroyActor` OtherActor)))

(event `/Game/Blueprints/Interfaces/BPI_Damageable.AddHealth`
  (params (HealingAmount :type "Float (double-precision)"))
  ; Add Health logic
  (set `self.Health` (`KismetMathLibrary.FClamp` (+ (`self.Health`) HealingAmount) 0.0 100.0)))

(event `WeaponFired`
  (if (== (`self.Current Weapon`) "/Game/Blueprints/Weapons/BP_Shovel.BP_Shovel")
    (set `self.Weapon2Fired` true)
    (`KismetSystemLibrary.Delay` 1.0)
    (set `self.Weapon2Fired` false)
    (else
      (set `self.Weapon1Fired` true)
      (`KismetSystemLibrary.Delay` 2.0)
      (set `self.Weapon1Fired` false))))

(fn `AddToLeaderboard`
  (params (CharacterToAdd :type "Actor Object Reference"))
  (bind _asbp_game_mode (cast `/Game/Levels/BP_GameMode` (`GameplayStatics.GetGameMode`)))
  (`KismetArrayLibrary.Array_Add` (`/Game/Levels/BP_GameMode.LeaderboardData` _asbp_game_mode) (make `/Game/Blueprints/Leaderboard/S_LeadboardEntry` (`KismetSystemLibrary.GetObjectName` CharacterToAdd))))

(fn `AnimatorUpdate`)

(fn `CurrentHealth`
  (returns (Float :type "Float (double-precision)"))
  (return (`self.Health`)))

(fn `GetCurrentWeapon`
  (returns (EquipedWeapon :type "/Game/Blueprints/Weapons/BP_WeaponBase Object Reference"))
  (return (`self.Current Weapon`)))

(fn `GetWeaponSocket`
  (returns (NewParam :type "Vector Structure"))
  (return (`SceneComponent.GetSocketLocation` (`self.Mesh`) "DBSocket")))

(fn `Initialise`
  ; Movement
  (set `self.Movement  Mult` 1)
  (set `CharacterMovementComponent.MaxWalkSpeed` 250.0 (`self.CharacterMovement`))
  ; Health
  (set `self.Health` 100.0)
  (`self.SpawnShovel`)
  (`self.AddToLeaderboard` self))

(fn `isDead`
  (returns (bDead :type Boolean))
  (return (<= (`self.Health`) 0.0)))

(fn `LeaderBoardUpdate`
  (params (`Killed Character` :type "Actor Object Reference") (KillerCharacter :type "Actor Object Reference"))
  (locals (KillerName :type String))
  (bind _returnvalue (`GameplayStatics.GetGameMode`))
  (`/Engine/EditorBlueprintResources/StandardMacros.IsValid` _returnvalue
    (:`Is Valid`
      (bind _asbp_game_mode (cast `/Game/Levels/BP_GameMode` _returnvalue))
      (set `local.KillerName` (`KismetSystemLibrary.GetObjectName` KillerCharacter))
      (bind _leaderboarddata (`/Game/Levels/BP_GameMode.LeaderboardData` _asbp_game_mode))
      (for (_array_element _array_index) _leaderboarddata
        (bind (_playername _kills) (break `/Game/Blueprints/Leaderboard/S_LeadboardEntry` _array_element))
        (if (`KismetStringLibrary.EqualEqual_StrStr` _playername (`local.KillerName`))
          (bind _result (`/Engine/EditorBlueprintResources/StandardMacros.IncrementInt` _kills)
            (:`  `
              (`KismetArrayLibrary.Array_Set` _leaderboarddata _array_index (make `/Game/Blueprints/Leaderboard/S_LeadboardEntry` "" _result))
              (break))))))))

(fn `Respawn`)

(fn `SpawnDBShotgun`
  (`self.K2_DestroyActor` (`self.Current Weapon`))
  (bind _returnvalue (`|SpawnActorFromClass` "/Game/Blueprints/Weapons/BP_Shotgun.BP_Shotgun_C" (`SceneComponent.GetSocketTransform` (`self.Mesh`) "DBSocket" "RTS_World") "Undefined" "MultiplyWithRoot" null null))
  (bind _output_get (set `self.ShotgunRef` _returnvalue))
  (`self.K2_AttachToComponent` _output_get (`self.Mesh`) "WeaponSocket" "SnapToTarget" "SnapToTarget" "SnapToTarget" true)
  (set `self.Current Weapon` (`self.ShotgunRef`))
  (set `self.UnlockedShotgun` true)
  (`SceneComponent.SetVisibility` (`Actor.RootComponent` (`self.Current Weapon`)) true true))

(fn `SpawnShovel`
  (if (`self.UnlockedShotgun`)
    (`self.K2_DestroyActor` (`self.Current Weapon`)))
  (bind _returnvalue (`|SpawnActorFromClass` "/Game/Blueprints/Weapons/BP_Shovel.BP_Shovel_C" (`SceneComponent.GetSocketTransform` (`self.Mesh`) "WeaponSocket" "RTS_World") "Undefined" "MultiplyWithRoot" null null))
  (`self.K2_AttachToComponent` _returnvalue (`self.Mesh`) "WeaponSocket" "SnapToTarget" "SnapToTarget" "SnapToTarget" true)
  (bind _output_get (set `self.ShovelRef` _returnvalue))
  (set `self.Current Weapon` _output_get)
  (`SceneComponent.SetVisibility` (`Actor.RootComponent` (`self.Current Weapon`)) true true))

(fn `UserConstructionScript`)