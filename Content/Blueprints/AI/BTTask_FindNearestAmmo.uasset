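; Behavior tree task that searches for the shotgun pickup nearest to the AI's controlled pawn.
; It loops over all BP_ShotgunPickup actors, keeping any closer than the stored ClosestDistance as ClosestPickup.
; It writes that pickup to the NearestAmmoPickup blackboard key only if ClosestDistance is below zero, which a measured distance never satisfies.
; The task always finishes successfully and never resets the stored distance within the graph.
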(event `self.ReceiveExecuteAI`
  (params (OwnerController :type "AIController Object Reference") (ControlledPawn :type "Pawn Object Reference"))
  (`GameplayStatics.GetAllActorsOfClass` "/Game/Prefabs/BP_ShotgunPickup.BP_ShotgunPickup_C")
  (for _array_element _
    (bind _returnvalue (`KismetMathLibrary.Vector_Distance` (`Actor.K2_GetActorLocation` _array_element) (`Actor.K2_GetActorLocation` (`Controller.K2_GetPawn` OwnerController))))
    (if (< _returnvalue (`self.closestDistance`))
      (set `self.closestDistance` _returnvalue)
      (set `self.ClosestPickup` _array_element)))
  (if (> 0.0 (`self.closestDistance`))
    (`BTFunctionLibrary.SetBlackboardValueAsObject` (make `BlackboardKeySelector` _ "NearestAmmoPickup" "/Script/AIModule.BlackboardKeyType_Object") (`self.ClosestPickup`)))
  (`self.FinishExecute` true))