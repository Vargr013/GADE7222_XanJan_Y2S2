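; Base weapon Blueprint that fires hitscan shots using line traces on the Visibility channel, with debug drawing.
; FireWeapon traces from the player camera along its forward vector and calls ApplyDamage.
; Fire traces between supplied points if CanFire allows, treating a MaxAmmo of -1 as unlimited.
; It sends damage through BPI_Damageable and decrements Ammo only when a damageable actor is hit.
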(event `FireWeapon`
  (bind _playercameramanager (`PlayerController.PlayerCameraManager` (`self.Player Ref`)))
  (bind _returnvalue (`PlayerCameraManager.GetCameraLocation` _playercameramanager))
  (set `self.Player Ref` (`GameplayStatics.GetPlayerController` 0))
  (bind _outhit (`KismetSystemLibrary.LineTraceSingle` _returnvalue (+ _returnvalue (* (`SceneComponent.GetForwardVector` (`PlayerCameraManager.TransformComponent` _playercameramanager)) (`self.Range`))) "TraceTypeQuery1" false (`|MakeArray` (`self.Player Ref`) :!type "Actor Object Reference") "ForDuration"))
  (`GameplayStatics.ApplyDamage` (`.HitActor` (`GameplayStatics.BreakHitResult` _outhit)) (`KismetMathLibrary.Conv_IntToDouble` (`self.Damage`))))

(event `/Game/Blueprints/Interfaces/BPI_Shootable.Fire`
  (params (StartLocation :type "Vector Structure") (TargetLocation :type "Vector Structure") (Shooter :type "Actor Object Reference"))
  (bind _canshoot (`self.CanFire`))
  (if _canshoot
    (bind (_outhit _returnvalue) (`KismetSystemLibrary.LineTraceSingle` StartLocation TargetLocation "TraceTypeQuery1" false (`|MakeArray` Shooter) "ForDuration"))
    (if _returnvalue
      (if (`KismetSystemLibrary.DoesImplementInterface` (`.HitActor` (`GameplayStatics.BreakHitResult` _outhit)) "/Game/Blueprints/Interfaces/BPI_Damageable.BPI_Damageable_C")
        (bind _damage (`self.GetWeaponDamage`))
        (message `/Game/Blueprints/Interfaces/BPI_Damageable.TakeDamage` (`.HitActor` (`GameplayStatics.BreakHitResult` _outhit)) _damage Shooter)
        (bind _result (`/Engine/EditorBlueprintResources/StandardMacros.DecrementInt` (`self.Ammo`))
          (:`  `
            (set `self.Ammo` _result)))))))

(fn `CanFire`
  (returns (CanShoot :type Boolean))
  (if (== (`self.MaxAmmo`) -1)
    (return true)
    (else
      (return (> (`self.Ammo`) 0)))))

(fn `GetCurrentAmmo`
  (returns (CurrentAmmo :type Integer))
  (return (`self.Ammo`)))

(fn `GetWeaponDamage`
  (returns (Damage :type "Float (double-precision)"))
  (return (`KismetMathLibrary.Conv_IntToDouble` (`self.Damage`))))

(fn `UserConstructionScript`)