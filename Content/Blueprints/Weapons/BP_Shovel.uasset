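; BP_Shovel is a shovel weapon Blueprint that specializes a parent weapon class.
; On BeginPlay it runs the parent setup, then overrides the Range and Damage values.
; FireWeapon defers entirely to the parent implementation, so the shovel adds no firing logic of its own.
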(event `self.ReceiveBeginPlay`
  (`parent.ReceiveBeginPlay`)
  (set `self.Range` 2500)
  (set `self.Damage` 3))

(event `self.FireWeapon`
  (`parent.FireWeapon`))

(fn `UserConstructionScript`
  (`parent.UserConstructionScript`))