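; BP_Shotgun is a shotgun weapon Blueprint that specializes a parent weapon class.
; On BeginPlay it runs the parent logic, then overrides range, damage and ammo capacity, starting with a full two-shot load.
; FireWeapon delegates to the parent's firing logic, then decrements ammo by one, with no ammo check or reload in this Blueprint.
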(event `self.ReceiveBeginPlay`
  (`parent.ReceiveBeginPlay`)
  (set `self.Range` 10000)
  (set `self.Damage` 12)
  (set `self.MaxAmmo` 2)
  (set `self.Ammo` 2))

(event `self.FireWeapon`
  (`parent.FireWeapon`)
  (bind _result (`/Engine/EditorBlueprintResources/StandardMacros.DecrementInt` (`self.Ammo`))
    (:`  `
      (set `self.Ammo` _result))))

(fn `UserConstructionScript`
  (`parent.UserConstructionScript`))